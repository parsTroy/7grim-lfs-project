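; Level-building tool actor that generates a straight stair or ramp mesh in its Construction Script, spanning to the StairDestination transform.
; The destination's distance picks one of four length variants from the set chosen by the UseStairs and UseFoundation flags.
; The mesh is scaled in X and Z by destination offset over its bounds, with width from the destination's Y scale.
; It takes CustomMaterial, or a dynamic instance driven by colour and roughness settings.
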(event EventBeginPlay)

(event Collision|EventActorBeginOverlap
  (params (OtherActor :type Actor%20Object%20Reference)))

(event EventTick
  (params (DeltaSeconds :type Float%20%28single-precision%29)))

(fn ConstructionScript
  (bind _stair_destination (Variables|Default|GetStair%20Destination))
  (bind _stair_destination_2 (Variables|Default|GetStair%20Destination))
  (bind _returnvalue (Math|Vector|VectorLength (.location _stair_destination_2)))
  (bind _returnvalue_2 (- _returnvalue 5e+01))
  (bind _returnvalue_3 (/ _returnvalue_2 2.5e+02))
  (bind _returnvalue_4 (Math|Float|Floor _returnvalue_3))
  (bind _returnvalue_5 (Math|Integer|Clamp(Integer) _returnvalue_4 0 3))
  (Variables|Default|SetNew%20Asset (select (Variables|Default|GetUse%20Stairs?) (select (Variables|Default|GetUse%20Foundation?) (Utilities|Select :Index _returnvalue_5 :Option%200 0 :Option%201 0 :Option%202 0 :Option%203 0) (Utilities|Select :Index _returnvalue_5 :Option%200 0 :Option%201 0 :Option%202 0 :Option%203 0)) (select (Variables|Default|GetUse%20Foundation?) (Utilities|Select :Index _returnvalue_5 :Option%200 0 :Option%201 0 :Option%202 0 :Option%203 0) (Utilities|Select :Index _returnvalue_5 :Option%200 0 :Option%201 0 :Option%202 0 :Option%203 0))))
  (bind _returnvalue_6 (AddComponent|AddStaticMeshComponent false (Math|Transform|MakeTransform "0, 0, 0" "0, 0, 0" (Math|Vector|MakeVector (/ (.x (.location _stair_destination)) (- (.x (.max (StaticMesh|GetBoundingBox (Variables|Default|GetNew%20Asset)))) (.x (.min (StaticMesh|GetBoundingBox (Variables|Default|GetNew%20Asset)))))) (.y (.scale _stair_destination)) (/ (.z (.location _stair_destination)) (- (.z (.max (StaticMesh|GetBoundingBox (Variables|Default|GetNew%20Asset)))) (.z (.min (StaticMesh|GetBoundingBox (Variables|Default|GetNew%20Asset))))))))))
  (Components|StaticMesh|SetStaticMesh _returnvalue_6 (Variables|Default|GetNew%20Asset))
  (Utilities|IsValid (Variables|Material|GetCustom%20Material)
    (:Is%20Valid
      (Rendering|Material|SetMaterial _returnvalue_6 0 (Variables|Material|GetCustom%20Material)))
    (:Is%20Not%20Valid
      (bind _returnvalue_7 (Rendering|Material|CreateDynamicMaterialInstance 0 "None" "None" :!class /Script/Engine.KismetMaterialLibrary))
      (Rendering|Material|SetMaterial _returnvalue_6 0 _returnvalue_7)
      (Rendering|Material|SetVectorParameterValue _returnvalue_7 "Diffuse Colour" (Variables|Material|GetSurface%20Colour) :!class /Script/Engine.MaterialInstanceDynamic)
      (Rendering|Material|SetScalarParameterValue _returnvalue_7 "Unique colour for top?" (Math|Conversions|ToFloat(Boolean) (Variables|Default|GetUnique%20colour%20for%20top?)) :!class /Script/Engine.MaterialInstanceDynamic)
      (Rendering|Material|SetVectorParameterValue _returnvalue_7 "Diffuse Colour - Top" (Variables|Material|GetTop%20Colour) :!class /Script/Engine.MaterialInstanceDynamic)
      (Rendering|Material|SetScalarParameterValue _returnvalue_7 "Roughness" (Variables|Material|GetMaterial%20Roughness%20Value) :!class /Script/Engine.MaterialInstanceDynamic))))