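; Barricade Blueprint that falls apart when interacted with.
; On the StartEventsonInteract event, it turns on physics simulation for its four static meshes and wakes their rigid bodies so the pieces can move.
; After a short delay it disables collision on all four pieces, so they no longer block anything.
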(event EventStartEventsonInteract
  (bind _staticmesh (Variables|Default|GetStaticMesh))
  (Physics|SetSimulatePhysics _staticmesh true)
  (Class|PrimitiveComponent|WakeAllRigidBodies _staticmesh)
  (Utilities|FlowControl|Delay 2.0)
  (Collision|SetCollisionEnabled (Variables|Default|GetStaticMesh) "NoCollision"))

(fn ConstructionScript
  (|CallParentFunction))