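; BP_ObjectiveMarker is an objective marker that can be toggled and signals when an optional box trigger is overlapped.
; The construction script either sizes the box or destroys it.
; While enabled, the first overlap broadcasts ObjectiveMarkerReached, then, if DisableOnReached is set, disables itself and enables NextObjectiveToEnable.
; That handoff clears the next marker's DisableOnReached, and ResetOnEnabled is empty.
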(event OnComponentBeginOverlap(Box)
  (params (OverlappedComponent :type Primitive%20Component%20Object%20Reference) (OtherActor :type Actor%20Object%20Reference) (OtherComp :type Primitive%20Component%20Object%20Reference) (OtherBodyIndex :type Integer) (bFromSweep :type Boolean) (SweepResult :type Hit%20Result%20Structure%20%28by%20ref%29))
  (bind _nextobjectivetoenable (Variables|ObjectiveMarker|GetNextObjectiveToEnable))
  (if (Variables|ObjectiveMarker|GetEnabled)
    (Utilities|FlowControl|DoOnce false
      (:Completed
        (Default|CallOnObjectiveMarkerReached)
        (if (and (Variables|ObjectiveMarker|GetEnabled) (Variables|ObjectiveMarker|GetDisableOnReached))
          (CallFunction|EnableObjectiveMarker false false)
          (Utilities|IsValid _nextobjectivetoenable
            (:Is%20Valid
              (CallFunction|EnableObjectiveMarker _nextobjectivetoenable true false))))))))

(event Custom|ResetOnEnabled)

(fn ConstructionScript
  (if (Variables|ObjectiveMarker|GetUseTrigger)
    (Components|Box|SetBoxExtent (Variables|Components|GetBox) (Variables|ObjectiveMarker|GetTriggerSize) true)
    (else
      (Components|DestroyComponent (Variables|Components|GetBox)))))

(fn EnableObjectiveMarker
  (params (Enable :type Boolean) (DisableOnReached :type Boolean))
  (Variables|ObjectiveMarker|SetEnabled Enable)
  (Variables|ObjectiveMarker|SetDisableOnReached DisableOnReached)
  (CallFunction|ResetonEnabled))